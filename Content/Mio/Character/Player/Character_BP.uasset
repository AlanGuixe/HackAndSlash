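; Player character Blueprint with camera-relative movement, jumping and a sword that can be drawn, sheathed and swung.
; BeginPlay spawns BP_Sword1 on the pelvis socket; WithdrawSword toggles CanAttack and re-attaches it between pelvis and weapon sockets after a delay.
; Attack briefly raises HitAttack while CanAttack is set.
; Mouse and stick axes drive controller yaw and clamped SpringArm rotation; Interaction and ResetForwardCamera only print debug strings.
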(event `self.ReceiveBeginPlay`
  ;[1 1 1] BEGIN PLAY
  (bind _returnvalue (`|SpawnActorFromClass` "/Game/Blueprints/BP_Sword1.BP_Sword1_C" (`SceneComponent.GetSocketTransform` (`self.Mesh`) "WeaponInPelvis" "RTS_World") "Undefined" "OverrideRootScale" null null))
  (bind _output_get (set `self.Sword` _returnvalue))
  (`self.K2_AttachToComponent` _output_get (`self.Mesh`) "WeaponInPelvis" "SnapToTarget" "SnapToTarget" "SnapToTarget" true))

(event `InputAxis|MouseRotate`
  (params (AxisValue :type "Float (single-precision)"))
  (bind (_returnvalue_roll _returnvalue_pitch _returnvalue_yaw) (`KismetMathLibrary.BreakRotator` (`self.GetControlRotation`)))
  (bind _springarm (`self.SpringArm`))
  (bind (_returnvalue_roll_2 _returnvalue_pitch_2) (`KismetMathLibrary.BreakRotator` (`SpringArmComponent.GetTargetRotation` _springarm)))
  ;[0.3663 0.1746 0.4072] Mouse Rotacion + Movimiento rotado
  (`self.AddControllerYawInput` AxisValue)
  (`SceneComponent.K2_SetRelativeRotation` _springarm (`KismetMathLibrary.MakeRotator` 0.0 _returnvalue_pitch_2 _returnvalue_yaw) false false))

(event `InputAxis|MoveForward`
  (params (AxisValue :type "Float (single-precision)"))
  ;[1 0 0] Movimiento
  (`self.AddMovementInput` (`KismetMathLibrary.GetForwardVector` (`KismetMathLibrary.MakeRotator` 0.0 0.0 (.yaw (`self.GetControlRotation`)))) AxisValue))

(event `InputAxis|MoveRight`
  (params (AxisValue :type "Float (single-precision)"))
  ;[1 0 0] Movimiento
  (`self.AddMovementInput` (`KismetMathLibrary.GetRightVector` (`KismetMathLibrary.MakeRotator` 0.0 0.0 (.yaw (`self.GetControlRotation`)))) AxisValue))

(event `InputAction|Jump`
  (params (Key :type "Key Structure"))
  ;[1 0 0] Movimiento
  (:`Pressed`
    (`self.Jump`)))

(event `InputAxis|CameraRotationY`
  (params (AxisValue :type "Float (single-precision)"))
  ;[0.8958 0.4268 1] StickRotation + Forward char
  (`SceneComponent.K2_SetRelativeRotation` (`self.SpringArm`) (`KismetMathLibrary.MakeRotator` 0.0 (`KismetMathLibrary.FClamp` (+ (* AxisValue -1.0) (.pitch (`SceneComponent.RelativeRotation` (`self.SpringArm`)))) -30.0 20.0) (`KismetMathLibrary.FClamp` (+ (.yaw (`SceneComponent.RelativeRotation` (`self.SpringArm`))) (stale `InputAxis|CameraRotationZ` AxisValue)) -180.0 180.0)) false false :!label _label))

(event `InputAction|Interaction`
  (params (Key :type "Key Structure"))
  ;[0.3313 0.9502 1] Interacciones
  (:`Pressed`
    (`KismetSystemLibrary.PrintString` "Anim_Interaction")))

(event `InputAxis|CameraRotationZ`
  (params (AxisValue :type "Float (single-precision)"))
  ;[0.8958 0.4268 1] StickRotation + Forward char
  (`self.AddControllerYawInput` AxisValue)
  (goto _label))

(event `InputAction|WithdrawSword`
  (params (Key :type "Key Structure"))
  ;[0.3313 0.9502 1] Interacciones
  (:`Released`
    (if (`self.canAttack`)
      (set `self.canAttack` false)
      (`KismetSystemLibrary.PrintString` "GuardarEspada")
      (`KismetSystemLibrary.Delay` 1.22)
      (`self.K2_AttachToComponent` (`self.Sword`) (`self.Mesh`) "WeaponInPelvis" "SnapToTarget" "SnapToTarget" "SnapToTarget" true)
      (else
        (set `self.canAttack` true)
        (`KismetSystemLibrary.PrintString` "PuedeAtacar")
        (`KismetSystemLibrary.Delay` 0.76)
        (`self.K2_AttachToComponent` (`self.Sword`) (`self.Mesh`) "WeaponSocket" "SnapToTarget" "SnapToTarget" "SnapToTarget" true)))))

(event `InputAction|ResetForwardCamera`
  (params (Key :type "Key Structure"))
  (:`Pressed`
    (if true
      (`KismetSystemLibrary.PrintString` "Igual")
      (else
        (`KismetSystemLibrary.PrintString` "no igual")))))

(event `InputAction|Attack`
  (params (Key :type "Key Structure"))
  ;[0.3313 0.9502 1] Interacciones
  (:`Pressed`
    (if (`self.canAttack`)
      (set `self.hitAttack` true)
      (`KismetSystemLibrary.PrintString` "Ataco")
      (`KismetSystemLibrary.Delay` 0.5)
      (set `self.hitAttack` false)
      (else
        (set `self.hitAttack` false)))))

(fn `UserConstructionScript`)