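; Enemy character that carries a sword and collapses into a ragdoll when its health runs out.
; BeginPlay spawns a BP_Sword1 at the mesh's WeaponSocket and snaps it to that socket.
; Tick polls Health and, at zero or below, turns on physics for the capsule and all mesh bodies from the root bone, with the capsule ignoring PhysicsBody collisions.
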(event `self.ReceiveBeginPlay`
  (bind _returnvalue (`|SpawnActorFromClass` "/Game/Blueprints/BP_Sword1.BP_Sword1_C" (`SceneComponent.GetSocketTransform` (`self.Mesh`) "WeaponSocket" "RTS_World") "Undefined" "OverrideRootScale" null null))
  (`self.K2_AttachToComponent` _returnvalue (`self.Mesh`) "WeaponSocket" "SnapToTarget" "SnapToTarget" "SnapToTarget" true))

(event `self.ReceiveTick`
  (params (DeltaSeconds :type "Float (single-precision)"))
  (bind _mesh (`self.Mesh`))
  (if (<= (`self.health`) 0.0)
    (`PrimitiveComponent.SetSimulatePhysics` (`self.CapsuleComponent`) true)
    (`PrimitiveComponent.SetCollisionResponseToChannel` (`self.CapsuleComponent`) "ECC_PhysicsBody" "ECR_Ignore")
    (`SkeletalMeshComponent.SetAllBodiesBelowSimulatePhysics` _mesh (`SkinnedMeshComponent.GetBoneName` _mesh 0) true true)))

(fn `UserConstructionScript`)