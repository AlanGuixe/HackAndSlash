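; BP_Sword1 is a sword actor that damages enemies it touches while the player is attacking.
; Its Box overlap casts the other actor to Enemy_BP and checks the player character's HitAttack flag before subtracting Damage from the enemy's Health.
; The remaining health prints to screen as debug output, and an unconnected Delay node is left in the graph.
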(event `self.Box.OnComponentBeginOverlap`
  (params (OverlappedComponent :type "PrimitiveComponent Object Reference") (OtherActor :type "Actor Object Reference") (OtherComp :type "PrimitiveComponent Object Reference") (OtherBodyIndex :type Integer) (bFromSweep :type Boolean) (SweepResult :type "HitResult Structure (by ref)"))
  (bind _asenemy_bp (cast `/Game/Mio/Character/Enemy/Enemy_BP` OtherActor))
  (bind _ascharacter_bp (cast `/Game/Mio/Character/Player/Character_BP` (`GameplayStatics.GetPlayerCharacter` 0)))
  (if (`/Game/Mio/Character/Player/Character_BP.hitAttack` _ascharacter_bp)
    (bind _output_get (set `/Game/Mio/Character/Enemy/Enemy_BP.health` (- (`/Game/Mio/Character/Enemy/Enemy_BP.health` _asenemy_bp) (`self.damage`)) _asenemy_bp))
    (`KismetSystemLibrary.PrintString` (`KismetStringLibrary.Concat_StrStr` "VidaEnemigo: " (`KismetStringLibrary.Conv_DoubleToString` _output_get)))))

(fn `UserConstructionScript`)